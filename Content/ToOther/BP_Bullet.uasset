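; BP_Bullet is a projectile that plays a sound on spawn and damages the KillDozer player on hit.
; SetDirection sets the projectile movement velocity from a given direction and the initial speed.
; When the projectile stops, a player who is attacking and facing it within a narrow 2D angle cone blocks it without damage; otherwise the player is damaged.
; The bullet then destroys itself, as it does on any non-player hit.
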(event `self.ReceiveBeginPlay`
  (`GameplayStatics.SpawnSound2D` "/Game/Sounds/Sound_Bullet.Sound_Bullet" 1.0 1.0 0.0 null))

(event `SetDirection`
  (params (Direction :type "Vector Structure"))
  (bind _projectilemovement (`self.ProjectileMovement`))
  (set `MovementComponent.Velocity` (* Direction (`ProjectileMovementComponent.InitialSpeed` _projectilemovement)) _projectilemovement))

(event `self.ProjectileMovement.OnProjectileStop`
  (params (ImpactResult :type "HitResult Structure (by ref)"))
  (bind (_bblockinghit _binitialoverlap _time _distance _location _impactpoint _normal _impactnormal _physmat _hitactor) (`GameplayStatics.BreakHitResult` ImpactResult))
  (`KismetSystemLibrary.PrintString` "Destryo")
  (if (`self.ActorHasTag` _hitactor "Player")
    (bind _asbp_kill_dozer_character (cast `/Game/PlayerKilldozer/PlayerBlueprints/BP_KillDozerCharacter` _hitactor)
      (:`then`
        (if (and (`/Game/PlayerKilldozer/PlayerBlueprints/BP_KillDozerCharacter.Attacking` _asbp_kill_dozer_character) (<= (`self.AngleBetweenVectors` (`self.GetActorForwardVector` _asbp_kill_dozer_character) (- (`self.K2_GetActorLocation`) (`self.K2_GetActorLocation` _asbp_kill_dozer_character))) 35.0))
          (`KismetSystemLibrary.PrintString` "PlayerFront")
          (`self.K2_DestroyActor`)
          (else
            (`/Game/PlayerKilldozer/PlayerBlueprints/BP_KillDozerCharacter.DamagePlayer` _asbp_kill_dozer_character 5.0)
            (`self.K2_DestroyActor`))))
      (:`CastFailed`
        (`KismetSystemLibrary.PrintString` "BP_Bullet: Failed to cast to KillDozerCharacter" true true (struct :`R` 1.0 :`G` 0.028544 :`A` 1.0) 10.0)))
    (else
      (`self.K2_DestroyActor`))))

(fn `AngleBetweenVectors`
  (params (Vec1 :type "Vector Structure") (Vec2 :type "Vector Structure"))
  (returns (Degrees :type "Float (double-precision)"))
  (bind _returnvalue (`KismetMathLibrary.Conv_VectorToVector2D` Vec2))
  (bind _returnvalue_2 (`KismetMathLibrary.Conv_VectorToVector2D` Vec1))
  (return (`KismetMathLibrary.DegAcos` (/ (`KismetMathLibrary.DotProduct2D` _returnvalue_2 _returnvalue) (* (`KismetMathLibrary.VSize2D` _returnvalue_2) (`KismetMathLibrary.VSize2D` _returnvalue))))))

(fn `UserConstructionScript`)