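; BP_ObjectManager tracks building destruction for the Killdozer player and shows it on an on-screen progress bar.
; On BeginPlay it counts the House Type Building 001 geometry collection actors as the total and creates the ProgresssBar widget.
; The BuildingDestroyed event sets the destroyed count to Points + 1, rather than incrementing it, and sends the clamped ratio to the widget.
; An older score and progress-bar branch is left unconnected.
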(event `self.ReceiveBeginPlay`
  ;[1 1 1] Begin play Object manager
  (bind _outactors (`GameplayStatics.GetAllActorsOfClass` "/Game/PlayerKilldozer/PlayerBlueprints/GC_House_Type_Buildig_001_Blueprint.GC_House_Type_Buildig_001_Blueprint_C"))
  (set `self.TotalBuildings` (`KismetArrayLibrary.Array_Length` _outactors))
  (bind _returnvalue (`|CreateWidget` "/Game/PlayerKilldozer/PlayerBlueprints/ProgresssBar.ProgresssBar_C"))
  (bind _output_get (set `self.ProgressBarWidget` _returnvalue))
  (`UserWidget.AddToViewport` _output_get 0))

(event `BuildingDestroyed`
  (params (Points :type Integer))
  ;[1 0.5608 0.4392] Building Destroyed Custom Event
  (set `self.DestroyedBuildings` (+ Points 1))
  (`/Game/PlayerKilldozer/PlayerBlueprints/ProgresssBar.UpdateProgress` (`self.ProgressBarWidget`) (`KismetMathLibrary.FClamp` (`KismetMathLibrary.SafeDivide` (`KismetMathLibrary.Conv_IntToDouble` (`self.DestroyedBuildings`)) (`KismetMathLibrary.Conv_IntToDouble` (`self.TotalBuildings`)))))
  (`KismetSystemLibrary.PrintString` "Progress Bar Received"))

(fn `UserConstructionScript`)