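; BP_Killdozer is the player's Killdozer Blueprint, handling forward and backward tank movement.
; MoveTank clamps the incoming axis value with the StopBackMove and StopFrontMove flags to block either direction; neither flag is set in these graphs.
; The result offsets the actor along its forward vector through a swept SetActorLocation, with no delta-time or speed scaling.
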(event `MoveTank`
  (params (`Axis Value` :type "Float (single-precision)"))
  (set `self.AxisVal` `Axis Value`)
  (if (`self.StopBackMove`)
    (set `self.AxisVal` (`KismetMathLibrary.FClamp` (`self.AxisVal`))))
  (if (`self.StopFront Move`)
    (set `self.AxisVal` (`KismetMathLibrary.FClamp` (`self.AxisVal`) -1.0 0.0)))
  (`self.K2_SetActorLocation` (+ (* (`self.AxisVal`) (`self.GetActorForwardVector`)) (`self.K2_GetActorLocation`)) true))

(fn `UserConstructionScript`)