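; Timer component, filed with the AI spawner, that counts up to a time limit and broadcasts TimerComplete.
; It can start on BeginPlay or through ResetAndStartTimer, then accumulates delta seconds on Tick while on.
; Repeatable timers restart on completion; others stay on, so they broadcast again every following tick.
; Tick also prints the current clock value every frame, even when the timer is off.
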(event `self.ReceiveBeginPlay`
  (if (`self.StartOn`)
    (`self.ResetAndStartTimer`)))

(event `self.ReceiveTick`
  (params (DeltaSeconds :type "Float (single-precision)"))
  (`KismetSystemLibrary.PrintString` (`KismetStringLibrary.Concat_StrStr` "Timer: " (`KismetStringLibrary.Conv_DoubleToString` (`self.TimeOnClock`))) true true (struct :`G` 0.66 :`B` 1.0 :`A` 1.0) 2.0 "Timer")
  (if (`self.IsOn`)
    (bind _output_get (set `self.TimeOnClock` (+ DeltaSeconds (`self.TimeOnClock`))))
    (if (>= _output_get (`self.TimeLimit`))
      (`self.TimerComplete`)
      (if (`self.Repeatable`)
        (`self.ResetAndStartTimer`)))))

(fn `ResetAndStartTimer`
  (set `self.IsOn` true)
  (set `self.TimeOnClock` 0.0))