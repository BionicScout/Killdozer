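; BP_AITank is an AI tank Character that feeds its distance from the player to its Blackboard.
; On BeginPlay it sets the max walk speed from its Speed variable and writes the distance to player pawn 0 into the DistanceFromPlayer key.
; Tick recomputes and rewrites that key every frame, with no other decision logic in the Blueprint.
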(event `self.ReceiveBeginPlay`
  (set `CharacterMovementComponent.MaxWalkSpeed` (`self.Speed`) (`self.CharacterMovement`))
  (`BlackboardComponent.SetValueAsFloat` (`AIBlueprintHelperLibrary.GetBlackboard` null) "DistanceFromPlayer" (`KismetMathLibrary.Vector_Distance` (`self.K2_GetActorLocation`) (`self.K2_GetActorLocation` (`GameplayStatics.GetPlayerPawn` 0)))))

(event `self.ReceiveTick`
  (params (DeltaSeconds :type "Float (single-precision)"))
  (`BlackboardComponent.SetValueAsFloat` (`AIBlueprintHelperLibrary.GetBlackboard` null) "DistanceFromPlayer" (`KismetMathLibrary.Vector_Distance` (`self.K2_GetActorLocation`) (`self.K2_GetActorLocation` (`GameplayStatics.GetPlayerPawn` 0)))))

(fn `UserConstructionScript`)